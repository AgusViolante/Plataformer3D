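; BP_EnemyBase is an enemy base Blueprint that walks forward only while it detects a surface below its probe point.
; Each tick, LineTraceFloor runs a short sphere trace on the Visibility channel from the LineTraceFloorPos component along the actor's downward axis.
; A hit adds forward movement input; a miss adds none, with no turning logic.
; The trace leaves debug drawing on and prints its result.
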(event EventTick
  (params (DeltaSeconds :type Float%20%28single-precision%29))
  (bind _floordetected (CallFunction|LineTraceFloor))
  (if _floordetected
    (Pawn|Input|AddMovementInput (Transformation|GetActorForwardVector) 1.0 false)))

(fn ConstructionScript)

(fn LineTraceFloor
  (bind _linetracefloorpos (Variables|Default|GetLineTraceFloorPos))
  (bind _returnvalue (Transformation|GetWorldLocation _linetracefloorpos))
  (bind _returnvalue_2 (Collision|SphereTraceByChannel _returnvalue (+ _returnvalue (* (Math|Vector|GetUpVector (Transformation|GetActorRotation)) -100)) 1e+01 "TraceTypeQuery1" false 0 "ForDuration"))
  (Development|PrintString (Utilities|String|ToString(Boolean) _returnvalue_2))
  (return _returnvalue_2))